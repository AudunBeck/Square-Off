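; Game mode for a local multiplayer, last-player-standing game with Tori_BP pawns.
; On BeginPlay it creates the game instance's number of players, spawning and possessing a pawn at each PlayerStart tagged with the player index.
; PlayerDead recounts dead players and calls the win event when one remains.
; StartGame saves ready pawns' elements to the game instance, then opens PrototypeMap.
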(event EventTick
  (params (DeltaSeconds :type Float%20%28single-precision%29))
  (bind _asgame_instance_bp (Utilities|Casting|CastToGameInstance_BP (Game|GetGameInstance)))
  (Variables|Default|SetMaxPlayerCount (Variables|/Game/Blueprints/GameInstance_BP.GameInstance_BP_C|GetnumberOfPlayers _asgame_instance_bp)))

(event EventPlayerDead
  (bind _array_element (Utilities|Array|ForEachLoopwithBreak (Variables|Default|GetPlayers))
    (:LoopBody
      (if (Variables|/Script/un_EZ.Tori|GetisDead _array_element)
        (Variables|Default|SetDeadPlayers (+ (Variables|Default|GetDeadPlayers) 1))
        (if (== (Variables|Default|GetMaxPlayerCount) (+ (Variables|Default|GetDeadPlayers) 1))
          (Default|CallPlayerWon))))
    (:Completed
      (Variables|Default|SetDeadPlayers 0))))

(event EventBeginPlay
  (CallFunction|GetPlayerStartPoints)
  (CallFunction|SpawnPlayers))

(fn ConstructionScript)

(fn GetPlayerStartPoints
  (bind _outactors (Actor|GetAllActorsOfClass "/Script/Engine.PlayerStart"))
  (Variables|Default|SetPlayerStartArray _outactors))

(fn SpawnPlayers
  (bind _asgame_instance_bp (Utilities|Casting|CastToGameInstance_BP (Game|GetGameInstance)))
  (Variables|Default|SetnumberOfSpawns (Variables|/Game/Blueprints/GameInstance_BP.GameInstance_BP_C|GetnumberOfPlayers _asgame_instance_bp))
  (for _index (range 0 (- (Variables|/Game/Blueprints/GameInstance_BP.GameInstance_BP_C|GetnumberOfPlayers _asgame_instance_bp) 1))
    (Variables|Default|SetIndex _index)
    (for _array_element (Variables|Default|GetPlayerStartArray)
      (if (Utilities|Name|Equal(Name) (Variables|/Script/Engine.PlayerStart|GetPlayerStartTag _array_element) (Utilities|String|StringToName (Utilities|String|ToString(Integer) (Variables|Default|GetIndex))))
        (Class|GameplayStatics|CreatePlayer (Variables|Default|GetIndex))
        (bind _returnvalue (Game|SpawnActorfromClass "/Game/Blueprints/Tori_BP.Tori_BP_C" (Transformation|GetActorTransform _array_element) "AlwaysSpawn" 0 0))
        (Pawn|Possess (Game|GetPlayerController (Variables|Default|GetIndex)) _returnvalue)
        (Utilities|Array|AddUnique (Variables|Default|GetPlayers) _returnvalue)))))

(fn StartGame
  (bind _outactors (Actor|GetAllActorsOfClass "/Game/Blueprints/Tori_BP.Tori_BP_C"))
  (for _array_element _outactors
    (if (Variables|/Game/Blueprints/Tori_BP.Tori_BP_C|GetisReady _array_element)
      (bind _returnvalue (Class|BaseElement|ReturnElementType (Variables|/Script/un_EZ.Tori|Getelement_1 _array_element)))
      (bind _asgame_instance_bp (Utilities|Casting|CastToGameInstance_BP (Game|GetGameInstance)))
      (Utilities|Array|Add (Variables|/Game/Blueprints/GameInstance_BP.GameInstance_BP_C|GetElementArray _asgame_instance_bp) _returnvalue)
      (Development|PrintString "Added element to list")))
  (Game|OpenLevel(byName) "PrototypeMap"))