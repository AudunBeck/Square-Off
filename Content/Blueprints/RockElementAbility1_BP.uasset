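; Actor for the first rock element ability, handling its audio and enemy hit effect.
; On BeginPlay it plays the ability sound through its Audio component.
; Overlapping a RockElementAbility2_BP stops that audio and calls PlaySoundAtLocation at the world origin, with no sound asset shown.
; HitEnemyVFX spawns the hit emitter at the given enemy location using the actor's rotation, then turns it a half turn.
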(event EventBeginPlay
  (Audio|Components|Audio|SetSound (Variables|Default|GetAudio) "/Game/Assets/Sound/RockAbility1.RockAbility1")
  (Audio|Components|Audio|Play (Variables|Default|GetAudio) 0.0))

(event Collision|EventActorBeginOverlap
  (params (OtherActor :type Actor%20Object%20Reference))
  (Utilities|Casting|CastToRockElementAbility2_BP OtherActor)
  (Audio|Components|Audio|Stop (Variables|Default|GetAudio))
  (Audio|PlaySoundatLocation 0 "0, 0, 0" "0, 0, 0" 1.0 1.0 0.0 0 0 0))

(event EventTick
  (params (DeltaSeconds :type Float%20%28single-precision%29)))

(event EventHitEnemyVFX
  (params (enemyLocation :type Vector :default "0, 0, 0"))
  (bind _returnvalue (Effects|SpawnEmitteratLocation (Variables|Default|GethitVFX) enemyLocation (Transformation|GetActorRotation)))
  (Transformation|AddWorldRotation _returnvalue "0,180.000000, 0" false false))

(fn ConstructionScript)