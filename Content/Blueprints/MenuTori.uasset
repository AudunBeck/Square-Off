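; MenuTori is the menu variant of a Tori actor, used to pick an element and ready up before a match.
; Each gamepad face button clears the current element, spawns a fire, rock or water pickup at the actor and sets IsReady; the wind button spawns fire as a placeholder.
; When CanPressStart is true, Start copies the ready count to the game mode's MaxPlayerCount and opens AudunPrototypeMap after a delay.
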(event EventBeginPlay
  (|CallParentFunction)
  (Variables|Default|SetisMenuTori true)
  (bind _asun_ezgame_mode_base_bp (Utilities|Casting|CastToun_EZGameModeBase_BP (Game|GetGameMode)))
  (Variables|Default|SetgameModeRef _asun_ezgame_mode_base_bp))

(event Collision|EventActorBeginOverlap
  (params (OtherActor :type Actor%20Object%20Reference))
  (|CallParentFunction OtherActor) ; This node is disabled and will not be called.\nDrag off pins to build functionality.
)

(event EventTick
  (params (DeltaSeconds :type Float%20%28single-precision%29))
  (|CallParentFunction DeltaSeconds) ; This node is disabled and will not be called.\nDrag off pins to build functionality.
)

(event Input|GamepadEvents|GamepadFaceButtonBottom
  (params (Key :type Key%20Structure))
  (:Pressed
    (Class|Tori|ClearElement)
    (Game|SpawnActorfromClass "/Game/Blueprints/pickUpWater_BP.pickUpWater_BP_C" (Transformation|GetActorTransform) "Undefined" 0 0)
    (Variables|Default|SetisReady true)))

(event Input|GamepadEvents|GamepadFaceButtonLeft
  (params (Key :type Key%20Structure))
  (:Pressed
    (Class|Tori|ClearElement)
    (Game|SpawnActorfromClass "/Game/Blueprints/pickUpRock_BP.pickUpRock_BP_C" (Transformation|GetActorTransform) "Undefined" 0 0)
    (Variables|Default|SetisReady true)))

(event Input|GamepadEvents|GamepadFaceButtonRight
  (params (Key :type Key%20Structure))
  (:Pressed
    (Class|Tori|ClearElement)
    (Game|SpawnActorfromClass "/Game/Blueprints/pickUpFire_BP.pickUpFire_BP_C" (Transformation|GetActorTransform) "Undefined" 0 0)
    (Variables|Default|SetisReady true)
    (Development|PrintString "Wind Element not functioning yet - Adding fire element instead")))

(event Input|GamepadEvents|GamepadFaceButtonTop
  (params (Key :type Key%20Structure))
  (:Pressed
    (Class|Tori|ClearElement)
    (Game|SpawnActorfromClass "/Game/Blueprints/pickUpFire_BP.pickUpFire_BP_C" (Transformation|GetActorTransform) "Undefined" 0 0)
    (Variables|Default|SetisReady true)))

(event Input|GamepadEvents|GamepadSpecialRight
  (params (Key :type Key%20Structure))
  (:Pressed
    (if (Variables|Default|GetcanPressStart)
      (Development|PrintString "Going to next level")
      (Variables|/Game/Blueprints/un_EZGameModeBase_BP.un_EZGameModeBase_BP_C|SetMaxPlayerCount (Variables|Default|GetgameModeRef) (Variables|Default|GetmenuToriNumReady))
      (Utilities|FlowControl|Delay 3.0)
      (Game|OpenLevel(byName) "AudunPrototypeMap")
      (else
        (Development|PrintString "Not enough players ready")))))

(fn ConstructionScript
  (|CallParentFunction))