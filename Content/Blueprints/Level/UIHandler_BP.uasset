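; Level actor that drives the multiplayer HUD: circular health bars and score indicators for up to four players.
; BeginPlay adds the HealthUI widget, creates per-player dynamic bar materials and caches component references and the game mode.
; Tick writes hit-point percentages to each bar's Alpha parameter.
; Events space out visible bars, shifting UICam for two players, and swap score particle templates from a flattened six-per-player array indexed by score.
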(event Custom|Update%20Score
  (params (PlayerNum :type Integer))
  (Effects|Components|ParticleSystem|SetTemplate (Utilities|Array|Get(acopy) (Variables|Default|GetScoreRefs1) PlayerNum) (Utilities|Array|Get(acopy) (Variables|Default|GetScoreParticles) (+ (* PlayerNum 6) (Utilities|Array|Get(acopy) (Variables|/Game/Blueprints/un_EZGameModeBase_BP.un_EZGameModeBase_BP_C|GetPlayerScores (Variables|Default|GetGameMode)) PlayerNum)))))

(event EventBeginPlay
  (bind _barrefs (Variables|Default|GetBarRefs))
  (bind _player2 (Variables|Default|GetPlayer2))
  (bind _player3 (Variables|Default|GetPlayer3))
  (bind _player4 (Variables|Default|GetPlayer4))
  (bind _player1 (Variables|Default|GetPlayer1))
  (bind _returnvalue (UserInterface|CreateWidget "/Game/UI/HealthUI.HealthUI_C"))
  (UserInterface|Viewport|AddtoViewport _returnvalue 0)
  (Rendering|Material|CreateDynamicMaterialInstance _player1 0 "/Game/UI/Materials/MI_circularHealthBar_player1.MI_circularHealthBar_player1" "None" :!class /Script/Engine.PrimitiveComponent)
  (Rendering|Material|CreateDynamicMaterialInstance _player2 0 "/Game/UI/Materials/MI_circularHealthBar_player2.MI_circularHealthBar_player2" "None" :!class /Script/Engine.PrimitiveComponent)
  (Rendering|Material|CreateDynamicMaterialInstance _player3 0 "/Game/UI/Materials/MI_circularHealthBar_player3.MI_circularHealthBar_player3" "None" :!class /Script/Engine.PrimitiveComponent)
  (Rendering|Material|CreateDynamicMaterialInstance _player4 0 "/Game/UI/Materials/MI_circularHealthBar_player4.MI_circularHealthBar_player4" "None" :!class /Script/Engine.PrimitiveComponent)
  (Utilities|Array|Add _barrefs _player1)
  (Utilities|Array|Add _barrefs _player2)
  (Utilities|Array|Add _barrefs _player3)
  (Utilities|Array|Add _barrefs _player4)
  (bind _asun_ezgame_mode_base_bp (Utilities|Casting|CastToun_EZGameModeBase_BP (Game|GetGameMode)))
  (Variables|Default|SetGameMode _asun_ezgame_mode_base_bp)
  (CallFunction|SetupScores))

(event EventTick
  (params (DeltaSeconds :type Float%20%28single-precision%29))
  (for _index (range 0 (- (Variables|Default|GetplayerAmount) 1))
    (Rendering|Material|SetScalarParameterValueonMaterials (Utilities|Array|Get(acopy) (Variables|Default|GetBarRefs) _index) "Alpha" (Utilities|Array|Get(acopy) (Variables|Default|GetplayersHitPointPercent) _index))))

(event EventSetBarPositions
  (bind _uicam (Variables|Default|GetUICam))
  (bind _playeramount (Variables|Default|GetplayerAmount))
  (bind _relativelocation (Variables|/Script/Engine.SceneComponent|GetRelativeLocation _uicam))
  (bind (_x _y _z) (Math|Vector|BreakVector _relativelocation))
  (for _index (range 0 (- _playeramount 1))
    (Rendering|SetVisibility (Utilities|Array|Get(acopy) (Variables|Default|GetBarRefs) _index) true true)
    (Transformation|SetRelativeLocation (Utilities|Array|Get(acopy) (Variables|Default|GetBarRefs) _index) (Math|Vector|MakeVector (* (+ _index 1) (Variables|Default|GetlengthBetween)) 0.0 0.0) false true)
    (Development|PrintString (Utilities|String|ToString(Float) (* (+ _index 1) (Variables|Default|GetlengthBetween)))))
  (if (== _playeramount 2)
    (Transformation|SetRelativeLocation _uicam (Math|Vector|MakeVector 1.8e+02 _y _z) false false)))

(fn ConstructionScript)

(fn SetUpPlayers)

(fn SetupScores
  (bind _scorerefs1 (Variables|Default|GetScoreRefs1))
  (Utilities|Array|Add _scorerefs1 (Variables|Default|GetParticleScore1))
  (Utilities|Array|Add _scorerefs1 (Variables|Default|GetParticleScore2))
  (Utilities|Array|Add _scorerefs1 (Variables|Default|GetParticleScore3))
  (Utilities|Array|Add _scorerefs1 (Variables|Default|GetParticleScore4)))