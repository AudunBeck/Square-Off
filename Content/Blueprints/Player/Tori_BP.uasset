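; Player character Blueprint for Tori, handling per-player colors, element-based Anim Blueprint switching, hit effects, scoring and death.
; Death helpers ragdoll the body with global slow motion; once IsDead, Tick hands the controller to a newly spawned ToriSpawner_BP, then destroys Tori.
; Exposed events cover dash montage, freeze frames, trace-based landing checks, dropping through platforms and hit flashes via timeline-driven dynamic materials.
; C triggers ragdoll death directly, and Escape opens the start menu.
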(event EventFreezeFrame
  (params (timeFrozen :type Float%20%28single-precision%29) (endAnim :type Boolean))
  ;[1 1 1] Freeze frame
  (CallFunction|FreezeStart)
  (Utilities|FlowControl|Delay timeFrozen)
  (CallFunction|FreezeEnd)
  (if endAnim
    (Animation|StopAnimMontage 0)))

(event EventTick
  (params (DeltaSeconds :type Float%20%28single-precision%29))
  ;[1 1 1] Unpossess Tori upon death, possess "Spawner-box"
  (if (Variables|Default|GetisDead)
    (Utilities|FlowControl|DoOnce false
      (:Completed
        (Utilities|FlowControl|Delay 3.0)
        (Pawn|UnPossess (Game|GetPlayerController (Variables|Default|GetPlayerNumber)))
        (bind _asun_ezgame_mode_base_bp (Utilities|Casting|CastToun_EZGameModeBase_BP (Game|GetGameMode)))
        (bind _returnvalue (Game|SpawnActorfromClass "/Game/Blueprints/Player/ToriSpawner_BP.ToriSpawner_BP_C" (Math|Transform|MakeTransform (Math|Vector|MakeVector 0.0 (Math|Random|RandomFloatinRange -1e+03 1e+03) (Variables|/Game/Blueprints/un_EZGameModeBase_BP.un_EZGameModeBase_BP_C|GetSpawnHeight _asun_ezgame_mode_base_bp))) "Undefined" 0 0))
        (Pawn|Possess (Game|GetPlayerController (Variables|Default|GetPlayerNumber)) _returnvalue)
        (Variables|/Game/Blueprints/Player/ToriSpawner_BP.ToriSpawner_BP_C|SetPlayerNumber _returnvalue (Variables|Default|GetPlayerNumber))
        (Utilities|FlowControl|Delay 3.0)
        (Actor|DestroyActor)))))

(event EventBeginPlay
  ;[1 1 1] Setup Tori
  (Collision|SetCollisionResponsetoChannel (Variables|Default|GetCapsuleComponent) "ECC_Pawn" "ECR_Block"))

(event EventSwitchAnimationElement
  (CallFunction|AnimationSwitcher))

(event EventStopAllVelocity
  (Variables|/Script/Engine.MovementComponent|SetVelocity (Variables|Character|GetCharacterMovement) "0, 0, 0"))

(event EventSlowMoDeath
  (params (slowMoEffect :type Float%20%28single-precision%29) (slowMoTime :type Float%20%28single-precision%29))
  ;[1 1 1] Death, ragdoll and slow motion.
  (CallFunction|SetRagdoll)
  (Utilities|Time|SetGlobalTimeDilation slowMoEffect)
  (Utilities|FlowControl|Delay (* slowMoTime slowMoEffect))
  (Utilities|Time|SetGlobalTimeDilation 1.0))

(event EventDashAnim
  (Animation|Montage|PlayMontage (Variables|Character|GetMesh) "/Game/Assets/Tori/NewAnim/ToriDash_Montage.ToriDash_Montage" 1.5))

(event EventGainPoint
  (bind _asun_ezgame_mode_base_bp (Utilities|Casting|CastToun_EZGameModeBase_BP (Game|GetGameMode)))
  (Default|UpdateGameStats _asun_ezgame_mode_base_bp (Variables|Default|GetPlayerNumber)))

(event EventStopCollision
  ;[1 1 1] Can move down throug platforms
  (Collision|SetCollisionResponsetoChannel (Variables|Default|GetCapsuleComponent) "ECC_GameTraceChannel1" "ECR_Ignore"))

(event EventCheckifLanded
  (bind _capsulecomponent (Variables|Default|GetCapsuleComponent))
  ;[1 1 1] Check if Tori is touching the ground
  (bind _outactors (Actor|GetAllActorsOfClass "Tori_BP_C"))
  (bind (_outhit _returnvalue) (Collision|LineTraceByChannel (Transformation|GetWorldLocation _capsulecomponent) (+ (Transformation|GetWorldLocation _capsulecomponent) "0, 0,-100.000000") "TraceTypeQuery1" false _outactors "None"))
  (if _returnvalue
    (Variables|Default|SetisJumping false)
    (if (Utilities|Enum|Equal(Enum) (Utilities|GetDisplayName (.hitactor _outhit)) "Floor")
      (Variables|Default|SetonSolidGround true)
      (else
        (Variables|Default|SetonSolidGround false)))
    (else
      (Variables|Default|SetisJumping true))))

(event EventTakeHitAnim
  (params (direction :type Vector :default "0, 0, 0"))
  ;[1 1 1] Add what should happen on hit here.
  (if (not (Variables|Default|GethitAnimImmune))
    (bind _returnvalue (Effects|SpawnEmitteratLocation "/Game/Assets/vfx_hit/Particle_player_take_damage_001.Particle_player_take_damage_001" (Transformation|GetActorLocation) (Math|Conversions|RotationFromXVector direction)))
    (Transformation|AddRelativeRotation _returnvalue "0,270.000000,0.000000" false false)
    (Animation|Montage|PlayMontage (Variables|Character|GetMesh) "/Game/Assets/Tori/NewAnim/ToriTakeDamage_Montage.ToriTakeDamage_Montage" 1.0 0.0 "Hit"
      (:then
        (bind _gethitblend (Timeline|getHitTimeline PlayFromStart)
          (:Update
            (Rendering|Material|SetScalarParameterValue (Variables|Default|GetdynamicM1) "Blend" _gethitblend :!class /Script/Engine.MaterialInstanceDynamic)))))))

(event Input|KeyboardEvents|Escape
  (params (Key :type Key%20Structure))
  (:Pressed
    (Game|OpenLevel(byName) "StartMenu")))

(event Input|KeyboardEvents|C
  (params (Key :type Key%20Structure))
  ;[1 1 1] Death, ragdoll and slow motion.
  (:Pressed
    (CallFunction|SetRagdoll)
    (Utilities|Time|SetGlobalTimeDilation (stale EventSlowMoDeath slowMoEffect))
    (Utilities|FlowControl|Delay (* (stale EventSlowMoDeath slowMoTime) (stale EventSlowMoDeath slowMoEffect)))
    (Utilities|Time|SetGlobalTimeDilation 1.0)))

(fn ConstructionScript
  (Class|SkinnedMeshComponent|SetMasterPoseComponent (Variables|Default|GetArms) (Variables|Character|GetMesh) false))

(fn AnimationSwitcher
  (bind _mesh (Variables|Character|GetMesh))
  (bind _output_get (Variables|Default|SetElementType (Variables|Default|GetcurrentElementType)))
  (switch int _output_get
    (:0
      (Components|SkeletalMesh|SetAnimInstanceClass _mesh "/Game/Assets/Tori/NewAnim/AnimTori_Bp.AnimTori_BP_C"))
    (:1
      (Components|SkeletalMesh|SetAnimInstanceClass _mesh "/Game/Assets/RockElement/NewAnim/AnimRock_BP.AnimRock_BP_C"))
    (:2
      (Components|SkeletalMesh|SetAnimInstanceClass _mesh "/Game/Assets/FireElement/NewAnim/AnimFire_BP.AnimFire_BP_C"))
    (:3
      (Components|SkeletalMesh|SetAnimInstanceClass _mesh "/Game/Assets/WaterElement/NewAnim/AnimWater_BP.AnimWater_BP_C"))
    (:4
      (Components|SkeletalMesh|SetAnimInstanceClass _mesh "/Game/Assets/WindElement/Animation/AnimWind_BP.AnimWind_BP_C"))))

(fn FreezeStart
  (bind _mesh (Variables|Character|GetMesh))
  (bind _returnvalue (Components|SkeletalMesh|GetAnimInstance _mesh))
  (Class|AnimInstance|MontagePause _returnvalue 0)
  (Class|Tori|SetMoveSpeed 0.0)
  (Class|Tori|SetRotationRate 0.0)
  (return _returnvalue))

(fn FreezeEnd
  (Class|AnimInstance|MontageResume (Components|SkeletalMesh|GetAnimInstance (Variables|Character|GetMesh)))
  (Class|Tori|SetMoveSpeed (Variables|Default|GetmoveSpeed))
  (Class|Tori|SetRotationRate (Variables|Default|GetrotationRate)))

(fn SetRagdoll
  (bind _arms (Variables|Default|GetArms))
  (bind _mesh (Variables|Character|GetMesh))
  (Collision|SetCollisionResponsetoAllChannels (Variables|Default|GetCapsuleComponent) "ECR_Ignore")
  (Transformation|DetachFromComponent _arms "KeepWorld" "KeepWorld" "KeepWorld" false)
  (Class|SkinnedMeshComponent|SetMasterPoseComponent _arms 0 false)
  (Collision|SetCollisionProfileName _mesh "Ragdoll" :!class /Script/Engine.PrimitiveComponent)
  (Components|Animation|SetAnimationMode _mesh "AnimationSingleNode")
  (Physics|SetSimulatePhysics _mesh true)
  (Pawn|UnPossess (Pawn|GetController)))

(fn SetColor
  (bind _mesh (Variables|Character|GetMesh))
  (bind _playernumber (Variables|Default|GetPlayerNumber))
  (bind _playercol (Variables|Default|GetPlayerCol))
  (bind _mesh_2 (Variables|Character|GetMesh))
  (bind _mesh_3 (Variables|Character|GetMesh))
  (bind _output (Utilities|Array|Get(acopy) _playercol _playernumber))
  (Rendering|Material|SetMaterial _mesh 4 _output)
  (Rendering|Material|SetMaterial _mesh 2 _output)
  (Rendering|SetCustomDepthStencilValue (Variables|Character|GetMesh) (+ _playernumber 1))
  (bind _returnvalue (Rendering|Material|CreateDynamicMaterialInstance _mesh_3 0 (Variables|Default|GetMBase1) "None" :!class /Script/Engine.PrimitiveComponent))
  (bind _output_get (Variables|Default|SetdynamicM0 _returnvalue))
  (Rendering|Material|SetMaterial _mesh_3 1 _output_get)
  (Rendering|Material|SetMaterial _mesh_3 6 _output_get)
  (bind _returnvalue_2 (Rendering|Material|CreateDynamicMaterialInstance _mesh_2 3 (Variables|Default|GetMBase2) "None" :!class /Script/Engine.PrimitiveComponent))
  (bind _output_get_2 (Variables|Default|SetdynamicM1 _returnvalue_2))
  (Rendering|Material|SetMaterial _mesh_2 5 _output_get_2)
  (Rendering|Material|SetMaterial _mesh_2 7 _output_get_2))