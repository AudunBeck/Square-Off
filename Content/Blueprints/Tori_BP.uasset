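; Tori_BP is the Blueprint for Tori, changing the mesh's animation set to match the current element.
; The SwitchAnimationElement event calls AnimationSwitcher, which reads CurrentElementType and swaps the Mesh's AnimInstance class between a base Tori Anim Blueprint and rock, fire, water and wind variants.
; The graphs contain no other active logic, and nothing here sets the element.
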(event EventBeginPlay)

(event Collision|EventActorBeginOverlap
  (params (OtherActor :type Actor%20Object%20Reference)))

(event EventTick
  (params (DeltaSeconds :type Float%20%28single-precision%29)))

(event EventSwitchAnimationElement
  (CallFunction|AnimationSwitcher))

(fn ConstructionScript)

(fn AnimationSwitcher
  (bind _mesh (Variables|Character|GetMesh))
  (bind _output_get (Variables|Default|SetElementType (Variables|Default|GetcurrentElementType)))
  (switch int _output_get
    (:0
      (Components|SkeletalMesh|SetAnimInstanceClass _mesh "/Game/Assets/Tori/Animation/AnimTori_BP.AnimTori_BP_C"))
    (:1
      (Components|SkeletalMesh|SetAnimInstanceClass _mesh "/Game/Assets/RockElement/Animation/AnimRock_BP.AnimRock_BP_C"))
    (:2
      (Components|SkeletalMesh|SetAnimInstanceClass _mesh "/Game/Assets/FireElement/Animation/AnimFire_BP.AnimFire_BP_C"))
    (:3
      (Components|SkeletalMesh|SetAnimInstanceClass _mesh "/Game/Assets/WaterElement/Animation/AnimWater_BP.AnimWater_BP_C"))
    (:4
      (Components|SkeletalMesh|SetAnimInstanceClass _mesh "/Game/Assets/WindElement/Animation/AnimWind_BP.AnimWind_BP_C"))))