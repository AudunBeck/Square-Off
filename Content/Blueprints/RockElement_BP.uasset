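; Rock element for the Tori character that swaps in rock arm meshes and materials when active and drives two montage-based abilities.
; Each ability is DoOnce-gated and locks the owner with snap rotation during its montage, while separate DoCode events call the fire code.
; Ability 1 branches montage sections into a punch or an early loop exit, and Tick toggles the charge sound from the Charging flag.
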(event Custom|Ability1DoCode
  ;[1 1 1] Ability 1 start animation and start code
  (Class|BaseElement|Ability1FireCode))

(event Custom|Ability2DoCode
  (bind _myowner (Variables|Default|GetmyOwner))
  ;[1 1 1] Ability 2 start animation and start code
  (Class|BaseElement|Ability2FireCode)
  (Utilities|FlowControl|DoOnce false) ; enters at Reset
)

(event EventBeginPlay
  (Audio|PlaySoundatLocation "/Game/Assets/Sound/RockAbility1.RockAbility1" "0, 0, 0" "0, 0, 0" 1.0 1.0 0.0 0 0 0)
  (Audio|Components|Audio|SetSound (Variables|Default|GetAudio) "/Game/Assets/Sound/RockAbility1.RockAbility1"))

(event EventSetActive
  (params (active :type Boolean))
  (bind _myowner (Variables|Default|GetmyOwner))
  (bind _arms (Variables|/Script/un_EZ.Tori|GetArms _myowner))
  (if active
    (Class|SkinnedMeshComponent|SetSkeletalMesh _arms "/Game/Assets/RockElement/NewMesh/Rock_ArmsLegs.Rock_ArmsLegs" true)
    (CallFunction|SetDynamicMaterial _arms _myowner)))

(event EventAbility1Anim
  (bind _myowner (Variables|Default|GetmyOwner))
  ;[1 1 1] Ability 1 start animation and start code
  (Utilities|FlowControl|DoOnce false :!label _label
    (:Completed
      (Animation|Montage|PlayMontage (Variables|/Script/Engine.Character|GetMesh _myowner) "/Game/Assets/RockElement/NewAnim/RockAbility1_Montage.RockAbility1_Montage"
        (:then
          (Variables|/Script/un_EZ.Tori|Setlocked _myowner true)
          (Variables|/Script/un_EZ.Tori|SetsnapRotation _myowner true))
        (:OnCompleted
          (Variables|/Script/un_EZ.Tori|Setlocked _myowner false :!label _label_2)
          (Class|Tori|SetMoveSpeed _myowner (Variables|/Script/un_EZ.Tori|GetmoveSpeed _myowner))
          (Class|Tori|SetRotationRate _myowner (Variables|/Script/un_EZ.Tori|GetrotationRate _myowner))
          (Variables|/Script/un_EZ.Tori|SetsnapRotation _myowner false)
          (if (not (Variables|Default|GetStartedPunch))
            (goto _label Reset)))
        (:OnInterrupted
          (goto _label_2))))))

(event EventAbility2Anim
  (bind _myowner (Variables|Default|GetmyOwner))
  ;[1 1 1] Ability 2 start animation and start code
  (Utilities|FlowControl|DoOnce false
    (:Completed
      (Animation|Montage|PlayMontage (Variables|/Script/Engine.Character|GetMesh _myowner) "/Game/Assets/RockElement/NewAnim/RockAbility2_Montage.RockAbility2_Montage"
        (:then
          (Variables|/Script/un_EZ.Tori|Setlocked _myowner true)
          (Variables|/Script/un_EZ.Tori|SetsnapRotation _myowner true))
        (:OnCompleted
          (Variables|/Script/un_EZ.Tori|Setlocked _myowner false :!label _label)
          (Class|Tori|SetMoveSpeed _myowner (Variables|/Script/un_EZ.Tori|GetmoveSpeed _myowner))
          (Class|Tori|SetRotationRate _myowner (Variables|/Script/un_EZ.Tori|GetrotationRate _myowner))
          (Variables|/Script/un_EZ.Tori|SetsnapRotation _myowner false))
        (:OnInterrupted
          (goto _label))))))

(event EventResetAbility1
  (bind _myowner (Variables|Default|GetmyOwner))
  ;[1 1 1] Ability 1 start animation and start code
  (Utilities|FlowControl|DoOnce false) ; enters at Reset
)

(event EventTick
  (params (DeltaSeconds :type Float%20%28single-precision%29))
  (bind _audio (Variables|Default|GetAudio))
  (if (Variables|Default|Getcharging)
    (Utilities|FlowControl|DoOnce false :!label _label
      (:Completed
        (Audio|Components|Audio|Play _audio 0.0)))
    (else
      (Audio|Components|Audio|Stop _audio)
      (goto _label Reset))))

(event EventResetAbility2
  (bind _myowner (Variables|Default|GetmyOwner))
  ;[1 1 1] Ability 2 start animation and start code
  (Utilities|FlowControl|DoOnce false) ; enters at Reset
)

(event EventAttachRockGlove)

(event EventAbility1PunchAnim
  (bind _myowner (Variables|Default|GetmyOwner))
  (bind _mesh (Variables|/Script/Engine.Character|GetMesh _myowner))
  ;[1 1 1] Ability 1 start animation and start code
  (Variables|Default|SetStartedPunch true)
  (Animation|Montage|PlayMontage _mesh "/Game/Assets/RockElement/NewAnim/RockAbility1_Montage.RockAbility1_Montage" 1.0 0.0 "Punch"
    (:OnCompleted
      _)
    (:OnInterrupted
      _))
  (Variables|Default|SetStartedPunch false)
  (Utilities|FlowControl|DoOnce false) ; enters at Reset
)

(event EventStopLoopAnim
  (bind _myowner (Variables|Default|GetmyOwner))
  (bind _mesh (Variables|/Script/Engine.Character|GetMesh _myowner))
  (bind _returnvalue (Components|SkeletalMesh|GetAnimInstance _mesh))
  (bind _returnvalue_2 (Animation|Montage|MontageGetCurrentSection _returnvalue "/Game/Assets/RockElement/NewAnim/RockAbility1_Montage.RockAbility1_Montage"))
  (if (Utilities|Name|Equal(Name) _returnvalue_2 "Loop")
    (Ability|Animation|MontageJumptoSection _returnvalue "End" "/Game/Assets/RockElement/NewAnim/RockAbility1_Montage.RockAbility1_Montage")
    (elif (Utilities|Name|Equal(Name) _returnvalue_2 "Start")
      (Class|AnimInstance|MontageSetNextSection _returnvalue "Start" "End" "/Game/Assets/RockElement/NewAnim/RockAbility1_Montage.RockAbility1_Montage"))))

(fn ConstructionScript)

(fn SetDynamicMaterial
  (params (Arms :type Primitive%20Component%20Object%20Reference) (Tori%20Ref :type Object%20Object%20Reference))
  (bind _astori_bp (Utilities|Casting|CastToTori_BP Tori%20Ref))
  (Rendering|Material|SetMaterial Arms 0 "/Game/Assets/RockElement/NewMesh/rock1.rock1")
  (Rendering|Material|SetMaterial Arms 1 (Variables|/Game/Blueprints/Tori_BP.Tori_BP_C|GetdynamicM1 _astori_bp))
  (Rendering|Material|SetMaterial Arms 2 (Variables|/Game/Blueprints/Tori_BP.Tori_BP_C|GetdynamicM0 _astori_bp)))