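; Fire element's first ability Blueprint, supplying sound and particle feedback for a punch attack with a buffed variant.
; BeginSound branches on Buffed: the buffed version spawns a rotated effect at the right foot socket, while the normal one attaches an effect to the left or right hand depending on FireChi.
; HitEnemyVFX spawns the impact effect at a supplied enemy location.
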(event EventBeginPlay)

(event Collision|EventActorBeginOverlap
  (params (OtherActor :type Actor%20Object%20Reference)))

(event EventTick
  (params (DeltaSeconds :type Float%20%28single-precision%29)))

(event EventHitEnemyVFX
  (params (enemyLocation :type Vector :default "0, 0, 0"))
  (Effects|SpawnEmitteratLocation (Variables|Default|GethitVFX) enemyLocation))

(event EventBeginSound
  (bind _myplayer (Variables|Default|GetmyPlayer))
  (bind _normalpunchvfx (Variables|Default|GetnormalPunchVFX))
  (bind _mesh (Variables|/Script/Engine.Character|GetMesh _myplayer))
  (if (Variables|Default|Getbuffed)
    (Audio|PlaySoundatLocation "/Game/Assets/Sound/FireAbility1Buffed.FireAbility1Buffed" "0, 0, 0" "0, 0, 0" 1.0 1.0 0.0 0 0 0)
    ;[1 1 1] Might need to go forward.
    (bind _returnvalue (Effects|SpawnEmitteratLocation (Variables|Default|GetbuffedPunchVFX) (Transformation|GetSocketLocation _mesh "RightFootSocket") (Transformation|GetActorRotation _myplayer)))
    (Transformation|AddLocalRotation _returnvalue "0.000000,270.000000,0.000000" false false)
    (else
      (Audio|PlaySoundatLocation "/Game/Assets/Sound/FireAbility1.FireAbility1" "0, 0, 0" "0, 0, 0" 1.0 1.0 0.0 0 0 0)
      (if (== (Variables|/Script/un_EZ.FireElement|GetfireChi (Variables|Default|GetmyElement)) 1)
        (Effects|SpawnEmitterAttached _normalpunchvfx _mesh "LeftHandSocket")
        (else
          (Effects|SpawnEmitterAttached _normalpunchvfx _mesh "RightHandSocket"))))))

(fn ConstructionScript)