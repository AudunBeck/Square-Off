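; Wind element ability actor that plays the wind punch particle effect for the player's current combo step.
; BeginPlay arms a one-shot flag, so the first Tick spawns a single emitter in front of and slightly above MyPlayer, aligned to the player's rotation with a yaw offset.
; MyElement's Combo value picks the effect: the first two hits share one particle, and the third uses a different, larger one.
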(event Collision|EventActorBeginOverlap
  (params (OtherActor :type Actor%20Object%20Reference)))

(event EventTick
  (params (DeltaSeconds :type Float%20%28single-precision%29))
  (bind _myplayer (Variables|Default|GetmyPlayer))
  (bind _myplayer_2 (Variables|Default|GetmyPlayer))
  (bind _returnvalue (Transformation|GetActorLocation _myplayer_2))
  (bind _returnvalue_2 (Transformation|GetActorForwardVector _myplayer_2))
  (bind _returnvalue_3 (Transformation|GetActorRotation _myplayer))
  (bind _returnvalue_4 (* _returnvalue_2 9e+01))
  (bind _returnvalue_5 (+ _returnvalue _returnvalue_4 "0.000000,0.000000,40.000000"))
  (if (Variables|Default|Gettest)
    (Variables|Default|Settest false)
    (switch int (Variables|/Script/un_EZ.WindElement|Getcombo (Variables|Default|GetmyElement))
      (:1
        (bind _returnvalue_6 (Effects|SpawnEmitteratLocation "/Game/Assets/WindElement/vfx/particle_wind_punch_001.particle_wind_punch_001" _returnvalue_5 _returnvalue_3 "2.000000,2.000000,2.000000" :!label _label))
        (Transformation|AddRelativeRotation _returnvalue_6 "270.000000, 0,0.000000" false false))
      (:2
        (goto _label))
      (:3
        (bind _returnvalue_7 (Effects|SpawnEmitteratLocation "/Game/Assets/WindElement/vfx/particle_wind_punch_002.particle_wind_punch_002" _returnvalue_5 _returnvalue_3 "2.500000,2.500000,2.500000"))
        (Transformation|AddRelativeRotation _returnvalue_7 "270.000000, 0,0.000000" false false)))))

(event EventBeginPlay
  (Variables|Default|Settest true))

(fn ConstructionScript)