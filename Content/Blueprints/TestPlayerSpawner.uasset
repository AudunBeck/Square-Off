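; TestPlayerSpawner is a test spawner that swaps its controller over to a freshly spawned Tori_BP character.
; Pressing M or the gamepad top face button spawns Tori_BP at the spawner's transform, has the spawner's controller possess it, then destroys the spawner.
; On BeginPlay it also prints the number of ToriController_BP actors in the world.
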(event EventBeginPlay
  (bind _outactors (Actor|GetAllActorsOfClass "/Game/Blueprints/ToriController_BP.ToriController_BP_C"))
  (Development|PrintString (Utilities|String|ToString(Integer) (Utilities|Array|Length _outactors))))

(event Collision|EventActorBeginOverlap
  (params (OtherActor :type Actor%20Object%20Reference)))

(event EventTick
  (params (DeltaSeconds :type Float%20%28single-precision%29)))

(event Input|KeyboardEvents|M
  (params (Key :type Key%20Structure))
  (:Pressed
    (bind _returnvalue (Game|SpawnActorfromClass "/Game/Blueprints/Tori_BP.Tori_BP_C" (Transformation|GetActorTransform) "Undefined" 0 0))
    (Pawn|Possess (Pawn|GetController) _returnvalue)
    (Actor|DestroyActor)))

(event Input|GamepadEvents|GamepadFaceButtonTop
  (params (Key :type Key%20Structure))
  (:Pressed
    (bind _returnvalue (Game|SpawnActorfromClass "/Game/Blueprints/Tori_BP.Tori_BP_C" (Transformation|GetActorTransform) "Undefined" 0 0))
    (Pawn|Possess (Pawn|GetController) _returnvalue)
    (Actor|DestroyActor)))

(fn ConstructionScript)