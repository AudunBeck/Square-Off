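; Wind element for a character, swapping in wind arm meshes and materials and attaching a chest burst effect when activated.
; Both abilities play montages behind DoOnce gates that lock the owner, with Ability 1 also snapping rotation and choosing a down or normal section.
; DoCode events call each ability's fire code.
; StopCollision lets pawns overlap the owner until a Tick-driven Delay restores blocking after Ability 2's lifespan.
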(event Custom|Ability1DoCode
  ;[1 1 1] Ability 1 start animation and start code
  (Variables|Default|Setability1Down (Utilities|Set|Contains (Variables|Default|GetDownAttackNames) (Animation|Montage|MontageGetCurrentSection (Components|SkeletalMesh|GetAnimInstance (Variables|/Script/Engine.Character|GetMesh (Variables|Default|GetmyOwner))) "/Game/Assets/WindElement/Animation/WindAbility1_Montage.WindAbility1_Montage")))
  (Class|BaseElement|Ability1FireCode)
  (Audio|PlaySoundatLocation "/Game/Assets/Sound/Wind/WindAbility1.WindAbility1" "0, 0, 0" "0, 0, 0" 1.0 1.0 0.0 0 0 0))

(event Custom|Ability2DoCode
  (bind _myowner (Variables|Default|GetmyOwner))
  ;[1 1 1] Ability 2 start animation and start code
  (Class|BaseElement|Ability2FireCode)
  (Utilities|FlowControl|DoOnce false) ; enters at Reset
)

(event EventBeginPlay)

(event EventSetActive
  (params (active :type Boolean))
  (bind _myowner (Variables|Default|GetmyOwner))
  (if active
    (Class|SkinnedMeshComponent|SetSkeletalMesh (Variables|/Script/un_EZ.Tori|GetArms _myowner) "/Game/Assets/WindElement/NewMesh/Wind_ArmsLegs.Wind_ArmsLegs" true)
    (Transformation|AttachComponentToComponent (Variables|Default|GetChestBurst) (Variables|/Script/Engine.Character|GetMesh _myowner) "wind_chest" "KeepRelative" "KeepRelative" "KeepRelative" true)
    (CallFunction|SetDynamicMaterial)))

(event EventAbility1Anim
  (bind _myowner (Variables|Default|GetmyOwner))
  ;[1 1 1] Ability 1 start animation and start code
  (Utilities|FlowControl|DoOnce false :!label _label
    (:Completed
      (if (Variables|Default|Getability1AnimDown)
        (Variables|Default|SetStartPos1 "RightD")
        (else
          (Variables|Default|SetStartPos1 "RightN")))
      (Animation|Montage|PlayMontage (Variables|/Script/Engine.Character|GetMesh _myowner) "/Game/Assets/WindElement/Animation/WindAbility1_Montage.WindAbility1_Montage" 1.0 0.0 (Variables|Default|GetStartPos1)
        (:then
          (Variables|/Script/un_EZ.Tori|Setlocked _myowner true)
          (Variables|/Script/un_EZ.Tori|SetsnapRotation _myowner true))
        (:OnCompleted
          (Variables|/Script/un_EZ.Tori|Setlocked _myowner false :!label _label_2)
          (Variables|/Script/un_EZ.Tori|SetsnapRotation _myowner false)
          (Variables|Default|Setcombo 0)
          (goto _label Reset))
        (:OnInterrupted
          (goto _label_2))))))

(event EventAbility2Anim
  (bind _myowner (Variables|Default|GetmyOwner))
  ;[1 1 1] Ability 2 start animation and start code
  (Utilities|FlowControl|DoOnce false :!label _label
    (:Completed
      (Animation|Montage|PlayMontage (Variables|/Script/Engine.Character|GetMesh _myowner) "/Game/Assets/WindElement/Animation/WindAbility2_Montage.WindAbility2_Montage"
        (:then
          (Variables|/Script/un_EZ.Tori|Setlocked _myowner true))
        (:OnCompleted
          (Variables|/Script/un_EZ.Tori|Setlocked _myowner false :!label _label_2)
          (goto _label Reset))
        (:OnInterrupted
          (goto _label_2))))))

(event EventResetAbility1
  (bind _myowner (Variables|Default|GetmyOwner))
  ;[1 1 1] Ability 1 start animation and start code
  (Utilities|FlowControl|DoOnce false) ; enters at Reset
)

(event EventTick
  (params (DeltaSeconds :type Float%20%28single-precision%29))
  (if (Variables|Default|Getability2Active)
    (Utilities|FlowControl|Delay (+ (Variables|Default|Getability2Lifespan) 0.5))
    (Collision|SetCollisionResponsetoChannel (Variables|/Script/Engine.Character|GetCapsuleComponent (Variables|Default|GetmyOwner)) "ECC_Pawn" "ECR_Block")
    (Variables|Default|Setability2Active false)))

(event EventResetAbility2
  (bind _myowner (Variables|Default|GetmyOwner))
  ;[1 1 1] Ability 2 start animation and start code
  (Utilities|FlowControl|DoOnce false) ; enters at Reset
)

(event EventAbility2PullAnim
  ;[1 1 1] Ability 2 start animation and start code
  (Animation|Montage|PlayMontage (Variables|/Script/Engine.Character|GetMesh (Variables|Default|GetmyOwner)) "/Game/Assets/WindElement/Animation/WindAbility2_Montage.WindAbility2_Montage"
    (:then
      (Audio|PlaySoundatLocation "/Game/Assets/Sound/Wind/WindAbility2.WindAbility2" "0, 0, 0" "0, 0, 0" 1.0 1.0 0.0 0 0 0))))

(event Collision|EventActorBeginOverlap
  (params (OtherActor :type Actor%20Object%20Reference)))

(event EventAbility2PullParticle
  (Components|Activation|Activate (Variables|Default|GetChestBurst) true))

(fn ConstructionScript)

(fn StopCollision
  (Collision|SetCollisionResponsetoChannel (Variables|/Script/Engine.Character|GetCapsuleComponent (Variables|Default|GetmyOwner)) "ECC_Pawn" "ECR_Overlap")
  (Variables|Default|Setability2Active true))

(fn SetDynamicMaterial
  (bind _myowner (Variables|Default|GetmyOwner))
  (bind _arms (Variables|/Script/un_EZ.Tori|GetArms _myowner))
  (bind _astori_bp (Utilities|Casting|CastToTori_BP _myowner))
  (Rendering|Material|SetMaterial _arms 2 "/Game/Assets/PickUp/PickUpWind/Meshcolor_wind_005.Meshcolor_wind_005")
  (Rendering|Material|SetMaterial _arms 1 (Variables|/Game/Blueprints/Player/Tori_BP.Tori_BP_C|GetdynamicM1 _astori_bp))
  (Rendering|Material|SetMaterial _arms 4 (Variables|/Game/Blueprints/Player/Tori_BP.Tori_BP_C|GetdynamicM1 _astori_bp))
  (Rendering|Material|SetMaterial _arms 0 (Variables|/Game/Blueprints/Player/Tori_BP.Tori_BP_C|GetdynamicM0 _astori_bp))
  (Rendering|Material|SetMaterial _arms 3 (Variables|/Game/Blueprints/Player/Tori_BP.Tori_BP_C|GetdynamicM0 _astori_bp)))