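; Wind element's first ability Blueprint, which spawns a wind punch particle effect matched to the current combo step.
; A flag set on BeginPlay makes the spawn run once, on the first Tick.
; Combo steps 1 and 2 share one emitter, while step 3 uses a second, larger one.
; The emitter appears ahead of and slightly above the player, oriented along Direction with a yaw correction.
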(event Collision|EventActorBeginOverlap
  (params (OtherActor :type Actor%20Object%20Reference)))

(event EventTick
  (params (DeltaSeconds :type Float%20%28single-precision%29))
  (bind _myplayer (Variables|Default|GetmyPlayer))
  (bind _direction (Variables|Default|Getdirection))
  (bind _direction_2 (Variables|Default|Getdirection))
  (bind _returnvalue (Transformation|GetActorLocation _myplayer))
  (bind _returnvalue_2 (* _direction 1.5e+02))
  (bind _returnvalue_3 (+ _returnvalue _returnvalue_2 "0.000000,0.000000,40.000000"))
  (if (Variables|Default|Gettest)
    (Variables|Default|Settest false)
    (switch int (Variables|/Script/un_EZ.WindElement|Getcombo (Variables|Default|GetmyElement))
      (:1
        (bind _returnvalue_4 (Effects|SpawnEmitteratLocation "/Game/Assets/WindElement/vfx/wind_punch_particle_001.wind_punch_particle_001" _returnvalue_3 (Math|Conversions|RotationFromXVector _direction_2) "2.000000,2.000000,2.000000" :!label _label))
        (Transformation|AddRelativeRotation _returnvalue_4 "270.000000, 0,0.000000" false false))
      (:2
        (goto _label))
      (:3
        (bind _returnvalue_5 (Effects|SpawnEmitteratLocation "/Game/Assets/WindElement/vfx/wind_punch_particle_002.wind_punch_particle_002" _returnvalue_3 (Math|Conversions|RotationFromXVector _direction_2) "2.500000,2.500000,2.500000"))
        (Transformation|AddRelativeRotation _returnvalue_5 "270.000000, 0,0.000000" false false)))))

(event EventBeginPlay
  (Variables|Default|Settest true))

(fn ConstructionScript)