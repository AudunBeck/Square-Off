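; FireElementAbility2_BP is an actor for the fire element's second ability, providing its sound and particle effect.
; On BeginPlay it plays the fire cue at the world origin and spawns an enlarged beam-hit emitter at the actor's transform, then yaws it.
; Tick moves the stored emitter to the actor's location each frame, so it follows without attachment.
; The graph holds no damage or overlap logic.
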(event EventBeginPlay
  (Audio|PlaySoundatLocation "/Game/Assets/Sound/Fire/FireAbility2p2_Cue.FireAbility2p2_Cue" "0, 0, 0" "0, 0, 0" 1.0 1.0 0.0 0 0 0)
  (bind _returnvalue (Effects|SpawnEmitteratLocation "/Game/Assets/FireElement/vfx/P_Beam_Hit.P_Beam_Hit" (Transformation|GetActorLocation) (Transformation|GetActorRotation) "2.000000,2.000000,2.000000"))
  (bind _output_get (Variables|Default|SetParticles _returnvalue))
  (Transformation|AddRelativeRotation _output_get "270.000000,0.000000,0.000000" false false))

(event Collision|EventActorBeginOverlap
  (params (OtherActor :type Actor%20Object%20Reference)))

(event EventTick
  (params (DeltaSeconds :type Float%20%28single-precision%29))
  (Transformation|SetWorldLocation (Variables|Default|GetParticles) (Transformation|GetActorLocation) false false))

(fn ConstructionScript)