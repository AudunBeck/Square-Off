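; Fire element Blueprint that gives its owning character a fire look and two fire abilities.
; SetActive swaps the owner's arm mesh and materials, reusing Tori_BP's dynamic materials.
; DoOnce-gated montages lock movement and snap rotation, with FireChi picking Ability 1's combo section and Ability 2 adding charge effect and sound.
; Separate events run the fire code, reset gates or release locks early on hit.
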(event Custom|Ability2DoCode
  ;[1 1 1] Ability 2 start animation and start code
  (Class|BaseElement|Ability2FireCode)
  (Components|Activation|Deactivate (Variables|Default|GetCharged1)))

(event Custom|Ability1DoCode
  ;[1 1 1] Ability 1 start animation and fire code when animation says
  (Class|BaseElement|Ability1FireCode))

(event EventBeginPlay)

(event Collision|EventActorBeginOverlap
  (params (OtherActor :type Actor%20Object%20Reference)))

(event EventAbility1Anim
  (bind _myowner (Variables|Default|GetmyOwner))
  ;[1 1 1] Ability 1 start animation and fire code when animation says
  (Utilities|FlowControl|DoOnce false :!label _label
    (:Completed
      (bind _section (CallFunction|ComboAnim))
      (Animation|Montage|PlayMontage (Variables|/Script/Engine.Character|GetMesh _myowner) "/Game/Assets/FireElement/NewAnim/FireAbility1_Montage.FireAbility1_Montage" 1.0 0.0 _section
        (:then
          (Variables|/Script/un_EZ.Tori|Setlocked _myowner true)
          (Variables|/Script/un_EZ.Tori|SetsnapRotation _myowner true))
        (:OnCompleted
          (Variables|/Script/un_EZ.Tori|Setlocked _myowner false :!label _label_2)
          (Variables|/Script/un_EZ.Tori|SetsnapRotation _myowner false)
          (goto _label Reset))
        (:OnInterrupted
          (goto _label_2))))))

(event EventAbility1HitAnim
  (bind _myowner (Variables|Default|GetmyOwner))
  (bind _myowner_2 (Variables|Default|GetmyOwner))
  ;[1 1 1] Ability 1 start animation and fire code when animation says
  (Variables|/Script/un_EZ.Tori|Setlocked _myowner_2 false)
  (Variables|/Script/un_EZ.Tori|SetmoveLocked _myowner_2 false)
  (Utilities|FlowControl|DoOnce false) ; enters at Reset
)

(event EventAbility2Anim
  (bind _myowner (Variables|Default|GetmyOwner))
  ;[1 1 1] Ability 2 start animation and start code
  (Utilities|FlowControl|DoOnce false :!label _label
    (:Completed
      (Animation|Montage|PlayMontage (Variables|/Script/Engine.Character|GetMesh _myowner) "/Game/Assets/FireElement/NewAnim/FireAbility2_Montage.FireAbility2_Montage"
        (:then
          (Variables|/Script/un_EZ.Tori|Setlocked _myowner true)
          (Components|Activation|Activate (Variables|Default|GetCharged1) false)
          (Variables|/Script/un_EZ.Tori|SetsnapRotation _myowner true)
          (Audio|PlaySoundatLocation "/Game/Assets/Sound/Fire/FireAbility2p1_Cue.FireAbility2p1_Cue" "0, 0, 0" "0, 0, 0" 1.0 1.0 0.0 0 0 0))
        (:OnCompleted
          (Variables|/Script/un_EZ.Tori|Setlocked _myowner false :!label _label_2)
          (Class|Tori|SetMoveSpeed _myowner (Variables|/Script/un_EZ.Tori|GetmoveSpeed _myowner))
          (Class|Tori|SetRotationRate _myowner (Variables|/Script/un_EZ.Tori|GetrotationRate _myowner))
          (Variables|/Script/un_EZ.Tori|SetsnapRotation _myowner false)
          (goto _label Reset))
        (:OnInterrupted
          (goto _label_2))))))

(event EventTick
  (params (DeltaSeconds :type Float%20%28single-precision%29)))

(event EventAbility2HitAnim
  (bind _myowner (Variables|Default|GetmyOwner))
  ;[1 1 1] Ability 2 start animation and start code
  (Variables|/Script/un_EZ.Tori|Setlocked _myowner false)
  (Variables|/Script/un_EZ.Tori|SetmoveLocked _myowner false))

(event EventResetAbility1
  (bind _myowner (Variables|Default|GetmyOwner))
  ;[1 1 1] Ability 1 start animation and fire code when animation says
  (Utilities|FlowControl|DoOnce false) ; enters at Reset
)

(event EventResetAbility2
  (bind _myowner (Variables|Default|GetmyOwner))
  ;[1 1 1] Ability 2 start animation and start code
  (Utilities|FlowControl|DoOnce false) ; enters at Reset
)

(event EventSetActive
  (params (active :type Boolean))
  (bind _myowner (Variables|Default|GetmyOwner))
  (bind _arms (Variables|/Script/un_EZ.Tori|GetArms _myowner))
  (if active
    (Class|SkinnedMeshComponent|SetSkeletalMesh _arms "/Game/Assets/FireElement/NewMesh/Fire_ArmsLegs.Fire_ArmsLegs" true)
    (CallFunction|SetDynamicMaterial _arms _myowner)))

(fn ConstructionScript)

(fn ComboAnim
  (switch int (Variables|Default|GetfireChi)
    (:0
      (return "1st"))
    (:1
      (return "2nd"))
    (:2
      (return "3rd"))))

(fn SetDynamicMaterial
  (params (Arms :type Primitive%20Component%20Object%20Reference) (Tori%20Ref :type Object%20Object%20Reference))
  (bind _astori_bp (Utilities|Casting|CastToTori_BP Tori%20Ref))
  (Rendering|Material|SetMaterial Arms 2 "/Game/Assets/FireElement/vfx/Fire_material_002.Fire_material_002")
  (Rendering|Material|SetMaterial Arms 0 (Variables|/Game/Blueprints/Player/Tori_BP.Tori_BP_C|GetdynamicM1 _astori_bp))
  (Rendering|Material|SetMaterial Arms 3 (Variables|/Game/Blueprints/Player/Tori_BP.Tori_BP_C|GetdynamicM1 _astori_bp))
  (Rendering|Material|SetMaterial Arms 1 (Variables|/Game/Blueprints/Player/Tori_BP.Tori_BP_C|GetdynamicM0 _astori_bp))
  (Rendering|Material|SetMaterial Arms 4 (Variables|/Game/Blueprints/Player/Tori_BP.Tori_BP_C|GetdynamicM0 _astori_bp)))