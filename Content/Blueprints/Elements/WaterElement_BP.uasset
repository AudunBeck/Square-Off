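; Water element Blueprint that gives its owner water arms and two montage-driven abilities.
; Activation swaps the arms mesh and applies water and Tori dynamic materials.
; Ability 1 plays a first or second combo section, while Ability 2 opens a counter stance with pawn-overlap collision and a separate counter animation with particles.
; DoOnce gates block re-triggering, montage callbacks restore owner state, and DoCode events call the fire functions.
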(event Custom|Ability1DoCode
  (bind _myowner (Variables|Default|GetmyOwner))
  (bind _mesh (Variables|/Script/Engine.Character|GetMesh _myowner))
  ;[1 1 1] Ability 1 start animation and start code, plays 2nd if used within certain timeframe.
  (Class|BaseElement|Ability1FireCode)
  (Variables|/Script/un_EZ.Tori|Setability1Used (Variables|Default|GetmyOwner) false)
  (Utilities|FlowControl|DoOnce false) ; enters at Reset
)

(event Custom|Ability2DoCode
  ;[1 1 1] Ability 2 start animation and start code
  (Class|BaseElement|Ability2FireCode))

(event EventBeginPlay)

(event EventSetActive
  (params (active :type Boolean))
  (if active
    (Class|SkinnedMeshComponent|SetSkeletalMesh (Variables|/Script/un_EZ.Tori|GetArms (Variables|Default|GetmyOwner)) "/Game/Assets/WaterElement/NewMesh/Water_ArmsLegs.Water_ArmsLegs" true)
    (CallFunction|SetDynamicMaterials)))

(event EventAbility1Anim
  (bind _myowner (Variables|Default|GetmyOwner))
  (bind _mesh (Variables|/Script/Engine.Character|GetMesh _myowner))
  ;[1 1 1] Ability 1 start animation and start code, plays 2nd if used within certain timeframe.
  (Utilities|FlowControl|DoOnce false
    (:Completed
      (if (Variables|Default|Getcombo)
        (Animation|Montage|PlayMontage _mesh "/Game/Assets/WaterElement/NewAnim/WaterAbility1_Montage.WaterAbility1_Montage" 1.0 0.0 "2nd"
          (:then
            (Variables|/Script/un_EZ.Tori|Setlocked _myowner true :!label _label)
            (Variables|/Script/un_EZ.Tori|SetsnapRotation _myowner true))
          (:OnCompleted
            (Variables|/Script/un_EZ.Tori|Setlocked _myowner false :!label _label_2)
            (Variables|/Script/un_EZ.Tori|SetsnapRotation _myowner false))
          (:OnInterrupted
            (goto _label_2)))
        (else
          (Animation|Montage|PlayMontage _mesh "/Game/Assets/WaterElement/NewAnim/WaterAbility1_Montage.WaterAbility1_Montage" 1.0 0.0 "1st"
            (:then
              (goto _label))
            (:OnCompleted
              (goto _label_2))
            (:OnInterrupted
              (goto _label_2))))))))

(event EventAbility2Anim
  (bind _myowner (Variables|Default|GetmyOwner))
  (bind _sphere (Variables|Default|GetSphere))
  (bind _capsulecomponent (Variables|/Script/Engine.Character|GetCapsuleComponent _myowner))
  ;[1 1 1] Ability 2 start animation and start code
  (Utilities|FlowControl|DoOnce false :!label _label
    (:Completed
      (Animation|Montage|PlayMontage (Variables|/Script/Engine.Character|GetMesh _myowner) "/Game/Assets/WaterElement/NewAnim/WaterAbility2_Montage.WaterAbility2_Montage" 1.0 0.0 ""
        (:then
          (Variables|/Script/un_EZ.Tori|Setlocked _myowner true)
          (Collision|SetCollisionResponsetoChannel _capsulecomponent "ECC_Pawn" "ECR_Overlap")
          (Collision|SetCollisionResponsetoChannel _sphere "ECC_Pawn" "ECR_Overlap")
          (Variables|Default|SetCountering true)
          (Variables|/Script/un_EZ.Tori|SetsnapRotation (Variables|Default|GetmyOwner) true))
        (:OnCompleted
          (Variables|/Script/un_EZ.Tori|Setlocked _myowner false :!label _label_2)
          (Variables|/Script/un_EZ.Tori|SetdamageMultiplier _myowner 1.0)
          (Class|Tori|SetMoveSpeed _myowner (Variables|/Script/un_EZ.Tori|GetmoveSpeed _myowner))
          (Class|Tori|SetRotationRate _myowner (Variables|/Script/un_EZ.Tori|GetrotationRate _myowner))
          (Variables|/Script/un_EZ.Tori|SetsnapRotation (Variables|Default|GetmyOwner) false)
          (Collision|SetCollisionResponsetoChannel _capsulecomponent "ECC_Pawn" "ECR_Block")
          (Collision|SetCollisionResponsetoChannel _sphere "ECC_Pawn" "ECR_Ignore")
          (Variables|Default|SetCountering false)
          (Variables|/Script/un_EZ.Tori|SethitAnimImmune (Variables|Default|GetmyOwner) false)
          (goto _label Reset))
        (:OnInterrupted
          (goto _label_2))))))

(event EventAbility2CounterAnim
  (bind _myowner (Variables|Default|GetmyOwner))
  (bind _myowner_2 (Variables|Default|GetmyOwner))
  (Animation|Montage|PlayMontage (Variables|/Script/Engine.Character|GetMesh _myowner) "/Game/Assets/WaterElement/NewAnim/WaterAbility2_Montage.WaterAbility2_Montage" 1.0 0.0 "Counter"
    (:then
      (Variables|/Script/un_EZ.Tori|SetdamageMultiplier _myowner 1.0)
      (bind _returnvalue (Effects|SpawnEmitteratLocation "/Game/Assets/WaterElement/vfx/Ability2/WaterAbility2_attack_ALTERNATIVE.WaterAbility2_attack_ALTERNATIVE" (Transformation|GetActorLocation _myowner_2) (Transformation|GetActorRotation _myowner_2)))
      (Transformation|AddRelativeRotation _returnvalue "0, 0, 0" false false))))

(event EventResetAbility1
  (bind _myowner (Variables|Default|GetmyOwner))
  (bind _mesh (Variables|/Script/Engine.Character|GetMesh _myowner))
  ;[1 1 1] Ability 1 start animation and start code, plays 2nd if used within certain timeframe.
  (Utilities|FlowControl|DoOnce false) ; enters at Reset
)

(event EventResetAbility2
  (bind _myowner (Variables|Default|GetmyOwner))
  (bind _sphere (Variables|Default|GetSphere))
  (bind _capsulecomponent (Variables|/Script/Engine.Character|GetCapsuleComponent _myowner))
  ;[1 1 1] Ability 2 start animation and start code
  (Utilities|FlowControl|DoOnce false) ; enters at Reset
)

(event Collision|EventActorBeginOverlap
  (params (OtherActor :type Actor%20Object%20Reference)))

(fn ConstructionScript)

(fn SetDynamicMaterials
  (bind _myowner (Variables|Default|GetmyOwner))
  (bind _arms (Variables|/Script/un_EZ.Tori|GetArms _myowner))
  (bind _astori_bp (Utilities|Casting|CastToTori_BP _myowner))
  (Rendering|Material|SetMaterial _arms 1 "/Game/Assets/WaterElement/vfx/Water_Material_001.Water_Material_001")
  (Rendering|Material|SetMaterial _arms 2 (Variables|/Game/Blueprints/Player/Tori_BP.Tori_BP_C|GetdynamicM1 _astori_bp))
  (Rendering|Material|SetMaterial _arms 3 (Variables|/Game/Blueprints/Player/Tori_BP.Tori_BP_C|GetdynamicM1 _astori_bp))
  (Rendering|Material|SetMaterial _arms 0 (Variables|/Game/Blueprints/Player/Tori_BP.Tori_BP_C|GetdynamicM0 _astori_bp))
  (Rendering|Material|SetMaterial _arms 4 (Variables|/Game/Blueprints/Player/Tori_BP.Tori_BP_C|GetdynamicM0 _astori_bp))
  (Rendering|Material|SetMaterial _arms 5 (Variables|/Game/Blueprints/Player/Tori_BP.Tori_BP_C|GetdynamicM0 _astori_bp)))