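; Rock wall actor spawned by the Rock element's second ability, with animated spawn-out, hit reaction and movement sound.
; Tick traces a short line downward, ignoring other walls of its class, to set IsTouchingGround, and loops a DoOnce to start or stop audio based on MovingTime.
; StartDestroy bursts particles and StartDespawn sinks the wall; both disable box collision and destroy the actor after their montage, while MoveAnim plays a hit montage.
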(event EventBeginPlay
  (Audio|Components|Audio|SetSound (Variables|Default|GetAudio) "/Game/Assets/Sound/Rock/Rock03_Cue.Rock03_Cue"))

(event Collision|EventActorBeginOverlap
  (params (OtherActor :type Actor%20Object%20Reference)))

(event EventTick
  (params (DeltaSeconds :type Float%20%28single-precision%29))
  (bind _audio (Variables|Default|GetAudio))
  (bind _rootcomponent (Variables|Transformation|GetRootComponent))
  (bind _outactors (Actor|GetAllActorsOfClass "RockElementAbility2_BP_C"))
  (bind _returnvalue (Collision|LineTraceByChannel (Transformation|GetWorldLocation _rootcomponent) (+ (Transformation|GetWorldLocation _rootcomponent) "0, 0,-70.000000") "TraceTypeQuery1" false _outactors "None"))
  (Variables|Default|SetisTouchingGround _returnvalue)
  (if (> (Variables|Default|GetmovingTime) 0.0)
    (Utilities|FlowControl|DoOnce false :!label _label
      (:Completed
        (Audio|Components|Audio|Play _audio 0.0)))
    (else
      (Audio|Components|Audio|Stop _audio)
      (goto _label Reset))))

(event EventStartDestroy
  (Effects|SpawnEmitteratLocation "/Game/Assets/RockElement/vfx/P_Rock_Punch_Hit.P_Rock_Punch_Hit" (Transformation|GetActorLocation) (Transformation|GetActorRotation))
  (Collision|SetCollisionEnabled (Variables|Default|GetBox) "NoCollision")
  (Animation|Montage|PlayMontage (Variables|Default|GetRockWall) "/Game/Assets/RockElement/Wall/Anim_RockWall_DeSpawn_Front_Montage.Anim_RockWall_DeSpawn_Front_Montage"
    (:OnCompleted
      (Actor|DestroyActor))))

(event EventMoveAnim
  (Animation|Montage|PlayMontage (Variables|Default|GetRockWall) "/Game/Assets/RockElement/Wall/Anim_RockWall_TakeAHit1_Montage.Anim_RockWall_TakeAHit1_Montage"))

(event EventStartDespawn
  (Collision|SetCollisionEnabled (Variables|Default|GetBox) "NoCollision")
  (Animation|Montage|PlayMontage (Variables|Default|GetRockWall) "/Game/Assets/RockElement/Wall/Anim_RockWall_DeSpawn_Down_Montage.Anim_RockWall_DeSpawn_Down_Montage"
    (:OnCompleted
      (Actor|DestroyActor))))

(fn ConstructionScript)