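; Wind element Blueprint that lets its owner temporarily pass through pawns as part of its second ability.
; StopCollision sets the owner capsule's Pawn collision response to Overlap and flags the ability as active.
; While that flag is set, Tick runs a Delay slightly longer than the buff duration, then restores Block and clears the flag.
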(event EventBeginPlay)

(event Collision|EventActorBeginOverlap
  (params (OtherActor :type Actor%20Object%20Reference)))

(event EventTick
  (params (DeltaSeconds :type Float%20%28single-precision%29))
  (if (Variables|Default|Getability2Active)
    (Utilities|FlowControl|Delay (+ (Variables|Default|GetbuffDur) 0.5))
    (Collision|SetCollisionResponsetoChannel (Variables|/Script/Engine.Character|GetCapsuleComponent (Variables|Default|GetmyOwner)) "ECC_Pawn" "ECR_Block")
    (Variables|Default|Setability2Active false)))

(fn ConstructionScript)

(fn StopCollision
  (Collision|SetCollisionResponsetoChannel (Variables|/Script/Engine.Character|GetCapsuleComponent (Variables|Default|GetmyOwner)) "ECC_Pawn" "ECR_Overlap")
  (Variables|Default|Setability2Active true))