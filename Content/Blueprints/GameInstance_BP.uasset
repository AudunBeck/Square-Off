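; Game instance Blueprint whose SetupToriFromMenu function gives each Tori_BP character in the level a starting element pickup.
; It caches all Tori actors in PlayerRef and matches each to ElementArray by index, so assignment follows GetAllActorsOfClass order.
; For a rock, fire, water or air value, it clears that Tori's element and spawns the matching pickup at its transform.
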(fn SetupTorifromMenu
  (bind _outactors (Actor|GetAllActorsOfClass "/Game/Blueprints/Tori_BP.Tori_BP_C"))
  (bind _output_get (Variables|Default|SetPlayerRef _outactors))
  (for (_array_element _array_index) _output_get
    (switch int (Utilities|Array|Get(acopy) (Variables|Default|GetElementArray) _array_index)
      (:1
        (Class|Tori|ClearElement _array_element)
        (Game|SpawnActorfromClass "/Game/Blueprints/pickUpRock_BP.pickUpRock_BP_C" (Transformation|GetActorTransform _array_element) "Undefined" 0 0))
      (:2
        (Class|Tori|ClearElement _array_element)
        (Game|SpawnActorfromClass "/Game/Blueprints/pickUpFire_BP.pickUpFire_BP_C" (Transformation|GetActorTransform _array_element) "Undefined" 0 0))
      (:3
        (Class|Tori|ClearElement _array_element)
        (Game|SpawnActorfromClass "/Game/Blueprints/pickUpWater_BP.pickUpWater_BP_C" (Transformation|GetActorTransform _array_element) "Undefined" 0 0))
      (:4
        (Class|Tori|ClearElement _array_element)
        (Game|SpawnActorfromClass "/Game/Blueprints/pickUpAir_BP.pickUpAir_BP_C" (Transformation|GetActorTransform _array_element) "Undefined" 0 0)))))