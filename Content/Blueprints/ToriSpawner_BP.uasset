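; Player-controlled spawner pawn that drops a player into the level as a Tori character at a chosen spot.
; On Ability_1, it traces downward, ignoring other spawners, and on a hit spawns Tori_BP there once, then transfers possession and player number.
; It also spawns an impact actor that checks for enemies, sets the Tori's material, then destroys itself.
; BeginPlay caches SpawnHeight from the game mode.
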(event EventBeginPlay
  (bind _asun_ezgame_mode_base_bp (Utilities|Casting|CastToun_EZGameModeBase_BP (Game|GetGameMode)))
  (Variables|Default|SetspawnHeight (Variables|/Game/Blueprints/un_EZGameModeBase_BP.un_EZGameModeBase_BP_C|GetSpawnHeight _asun_ezgame_mode_base_bp)))

(event Collision|EventActorBeginOverlap
  (params (OtherActor :type Actor%20Object%20Reference)))

(event EventTick
  (params (DeltaSeconds :type Float%20%28single-precision%29)))

(event Input|ActionEvents|InputActionAbility_1
  (params (Key :type Key%20Structure))
  (bind _rootcomponent (Variables|Transformation|GetRootComponent))
  (:Pressed
    (bind _outactors (Actor|GetAllActorsOfClass "ToriSpawner_BP_C"))
    (bind (_outhit _returnvalue) (Collision|LineTraceByChannel (Transformation|GetWorldLocation _rootcomponent) (+ (Transformation|GetWorldLocation _rootcomponent) "0, 0,-1000.000000") "TraceTypeQuery1" true _outactors "ForOneFrame"))
    (if _returnvalue
      (Utilities|FlowControl|DoOnce false
        (:Completed
          (Pawn|UnPossess (Game|GetPlayerController (Variables|Default|GetPlayerNumber)))
          (bind _returnvalue_2 (Game|SpawnActorfromClass "/Game/Blueprints/Tori_BP.Tori_BP_C" (Math|Transform|MakeTransform (+ (.location _outhit) "0, 0,50.000000") "0,180.000000, 0") "Undefined" 0 0))
          (Pawn|Possess (Game|GetPlayerController (Variables|Default|GetPlayerNumber)) _returnvalue_2)
          (Variables|/Script/un_EZ.Tori|SetPlayerNumber _returnvalue_2 (Variables|Default|GetPlayerNumber))
          (bind _returnvalue_3 (Game|SpawnActorfromClass "/Game/Blueprints/SpawnInpact_BP.SpawnInpact_BP_C" (Math|Transform|MakeTransform (+ (.location _outhit) "0, 0,50.000000") "0,180.000000, 0") "Undefined" 0 0))
          (Class|SpawnInpact|CheckforEnemies _returnvalue_3 _returnvalue_2)
          (CallFunction|SetPlayerMaterial _returnvalue_2)
          (Actor|DestroyActor))))))

(fn ConstructionScript)

(fn SetPlayerMaterial
  (params (Player :type Character%20Object%20Reference))
  (bind _mesh (Variables|/Script/Engine.Character|GetMesh Player))
  (switch int 0
    (:0
      (Rendering|Material|SetMaterial _mesh 0 0))
    (:1
      (Rendering|Material|SetMaterial _mesh 0 0))
    (:2
      (Rendering|Material|SetMaterial _mesh 0 0))
    (:3
      (Rendering|Material|SetMaterial _mesh 0 0))))